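; Utility functions for a mixed reality project using MRUK: Android permissions, surface placement and navmesh fitting.
; Permission requests fire only when the permission is not already granted.
; Surface placement picks a random point on top of a labeled surface, else any surface, aligning Z to the normal, or X in the fallback.
; Navmesh fitting scales and centers a bounds volume on the current room with a margin, then notifies navigation.
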(fn RequestAndroidPermissionifNotGranted
  (params (Permission :type String))
  (bind _returnvalue (Class|AndroidPermissionFunctionLibrary|CheckPermission Permission))
  (if (not _returnvalue)
    (Class|AndroidPermissionFunctionLibrary|AcquirePermissions (Utilities|Array|MakeArray Permission))))

(fn GetLocationonSurfaceorAny
  (params (SemanticLabel :type String) (DistanceToEdge :type Float%20%28double-precision%29))
  (bind _returnvalue (Subsystems|GetMRUKSubsystem))
  (bind _returnvalue_2 (Class|MRUKSubsystem|GetCurrentRoom _returnvalue))
  (bind (_outposition _outnormal _returnvalue_3) (Class|MRUKRoom|GenerateRandomPositiononSurface _returnvalue_2 "OnTopOfSurface" DistanceToEdge (Utilities|Struct|MakeMRUKLabelFilter (Utilities|Array|MakeArray SemanticLabel))))
  (if _returnvalue_3
    (return (Math|Transform|MakeTransform _outposition (Math|Rotator|MakeRotfromZ _outnormal)))
    (else
      (bind (_outposition_2 _outnormal_2) (Class|MRUKRoom|GenerateRandomPositiononSurface _returnvalue_2 "OnTopOfSurface" DistanceToEdge))
      (return (Math|Transform|MakeTransform _outposition_2 (Math|Conversions|RotationFromXVector _outnormal_2))))))

(fn AdjustNavMeshBounds
  (params (NavMeshBoundsVolume :type Nav%20Mesh%20Bounds%20Volume%20Object%20Reference))
  (Utilities|IsValid (Class|MRUKSubsystem|GetCurrentRoom (Subsystems|GetMRUKSubsystem))
    (:Is%20Valid
      (LocalVariables|SetRoomBounds (Variables|/Script/MRUtilityKit.MRUKRoom|GetRoomBounds (Class|MRUKSubsystem|GetCurrentRoom (Subsystems|GetMRUKSubsystem))))
      (Transformation|SetActorScale3D NavMeshBoundsVolume (+ (/ (- (.max (LocalVariables|GetRoomBounds)) (.min (LocalVariables|GetRoomBounds))) 2.0) 1.0))
      (Transformation|SetActorLocation NavMeshBoundsVolume (/ (+ (.min (LocalVariables|GetRoomBounds)) (.max (LocalVariables|GetRoomBounds))) 2.0) false false)
      (Class|NavigationSystemV1|OnNavigationBoundsUpdated (Class|NavigationSystemV1|GetNavigationSystem) NavMeshBoundsVolume))))