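; Splash screen actor for a VR game that shows a logo widget over optional Meta XR persistent passthrough while the next level loads.
; It snaps to the headset camera and scales the widget from FOV and distance to fill a set screen fraction.
; After a minimum duration it fades out and removes passthrough.
; It then either opens the level directly or reveals an async-loaded, hidden level instance and destroys itself.
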(event Custom|OnLevelLoaded
  ;[0.03434 0.03434 0.03434] On timer finished & Level done loading
  (CallFunction|ShowLevelInstance))

(event Custom|OnLevelShown
  ;[0.03434 0.03434 0.03434] On timer finished & Level done loading
  (Utilities|FlowControl|Delay 0.0)
  (Actor|DestroyActor))

(event Custom|TimerFinished
  (bind _levelinstance (Variables|NextLevel|GetLevelInstance))
  ;[0.03434 0.03434 0.03434] On timer finished & Level done loading
  (if (Variables|NextLevel|GetAsyncLoadLevel)
    (if (Class|LevelStreaming|IsLevelLoaded _levelinstance)
      (CallFunction|ShowLevelInstance)
      (else
        (EventDispatchers|AssignOnLevelLoaded _levelinstance (delegate Custom|OnLevelLoaded))))
    (else
      (Default|PlayFadeOut (Variables|Default|GetSplashScreenWidget))
      (Utilities|FlowControl|Delay (Variables|SplashSettings|GetLogoFadeDuration))
      (Class|OculusXRPassthroughSubsystem|DestroyPersistentPassthrough (Subsystems|GetOculusXRPassthroughSubsystem))
      (Game|OpenLevel(byObjectReference) (Variables|NextLevel|GetLevelToLoad)))))

(event Custom|ShowLevelInstance
  (bind _levelinstance (Variables|NextLevel|GetLevelInstance))
  ;[0.03434 0.03434 0.03434] On timer finished & Level done loading
  (Default|PlayFadeOut (Variables|Default|GetSplashScreenWidget))
  (Utilities|FlowControl|Delay (Variables|SplashSettings|GetLogoFadeDuration))
  (Class|OculusXRPassthroughSubsystem|DestroyPersistentPassthrough (Subsystems|GetOculusXRPassthroughSubsystem))
  (EventDispatchers|AssignOnLevelShown _levelinstance (delegate Custom|OnLevelShown))
  (Variables|/Script/Engine.LevelStreaming|SetbShouldBeVisible _levelinstance true))

(event EventBeginPlay
  (Utilities|FlowControl|Sequence
    (:then_0
      ;[0.03434 0.03434 0.03434] Check CTXPT
      (bind _returnvalue (Class|OculusXRFunctionLibrary|IsPassthroughRecommended))
      (if _returnvalue
        (Class|OculusXRPassthroughSubsystem|InitializePersistentPassthrough (Subsystems|GetOculusXRPassthroughSubsystem))))
    (:then_1
      ;[0.03434 0.03434 0.03434] Attach to headset camera
      (Transformation|AttachComponentToComponent (Actor|GetComponentbyClass (Game|Player|GetPlayerPawn 0) "/Script/Engine.CameraComponent") "None" "SnapToTarget" "SnapToTarget" "SnapToTarget" true)
      (CallFunction|UpdateWidgetTransform))
    (:then_2
      ;[0.03434 0.03434 0.03434] Start async loading
      (if (Variables|NextLevel|GetAsyncLoadLevel)
        (bind _returnvalue_2 (Class|LevelStreamingDynamic|LoadLevelInstancebySoftObjectPtr (Variables|NextLevel|GetLevelToLoad) "0, 0, 0" "0, 0, 0" "" 0 false))
        (bind _output_get (Variables|NextLevel|SetLevelInstance _returnvalue_2))
        (Variables|/Script/Engine.LevelStreaming|SetbShouldBeVisible _output_get false)))
    (:then_3
      ;[0.03434 0.03434 0.03434] Init widget
      (bind _asw_splash_screen (Utilities|Casting|CastToW_SplashScreen (UserInterface|GetWidget (Variables|Default|GetWidget))))
      (bind _output_get_2 (Variables|Default|SetSplashScreenWidget _asw_splash_screen))
      (Default|Init _output_get_2 (Variables|SplashSettings|GetMinDuration) (Variables|NextLevel|GetLevelInstance) (Variables|SplashSettings|GetLogoFadeDuration)))
    (:then_4
      ;[0.03434 0.03434 0.03434] Start timer
      (Utilities|FlowControl|Delay (Variables|SplashSettings|GetMinDuration))
      (CallFunction|TimerFinished))))

(fn ConstructionScript
  (CallFunction|UpdateWidgetTransform))

(fn UpdateWidgetTransform
  (bind _returnvalue (Game|GetPlayerCameraManager 0))
  (bind _returnvalue_2 (Camera|GetFOVAngle _returnvalue))
  (Variables|/Script/Engine.SpringArmComponent|SetTargetArmLength (Variables|Default|GetSpringArm) (* (Variables|SplashSettings|GetDistance) -1.0))
  (LocalVariables|SetDesiredWidth (* (/ (Variables|SplashSettings|GetDistance) (Math|Trig|Tan(Degrees) (* (select (== _returnvalue_2 0.0) (Variables|/Script/Engine.CameraComponent|GetFieldOfView (Variables|Default|GetCamera)) _returnvalue_2) 0.5))) 2.0 (Variables|SplashSettings|GetScreenPercentage)))
  (Class|WidgetComponent|SetDrawSize (Variables|Default|GetWidget) (Math|Conversions|ToVector2D(Vector) (Variables|SplashSettings|GetPixelSize)))
  (Transformation|SetWorldScale3D (Variables|Default|GetScalePivot) (Math|Conversions|ToVector(Float) (/ (LocalVariables|GetDesiredWidth) (Variables|SplashSettings|GetPixelSize)))))